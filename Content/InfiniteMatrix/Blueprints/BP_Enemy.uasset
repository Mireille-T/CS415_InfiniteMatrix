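; BP_Enemy is an enemy actor that damages the player on contact and awards score when a projectile hits it.
; All logic runs from its static mesh's begin-overlap event, which casts the other actor to tell player from projectile.
; A player hit lowers health, then shows restart at zero or otherwise disables the mesh's collision.
; A projectile hit updates the player's score and UI via GetActorOfClass, then destroys the enemy.
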(event `self.StaticMeshComponent.OnComponentBeginOverlap`
  (params (OverlappedComponent :type "PrimitiveComponent Object Reference") (OtherActor :type "Actor Object Reference") (OtherComp :type "PrimitiveComponent Object Reference") (OtherBodyIndex :type Integer) (bFromSweep :type Boolean) (SweepResult :type "HitResult Structure (by ref)"))
  (bind _asbp_player (cast `/Game/InfiniteMatrix/Blueprints/BP_Player` OtherActor)
    (:`then`
      (bind _output_get (set `/Game/InfiniteMatrix/Blueprints/BP_Player.PlayerHealth` (- (`/Game/InfiniteMatrix/Blueprints/BP_Player.PlayerHealth` _asbp_player) 1) _asbp_player))
      (`/Game/InfiniteMatrix/Blueprints/BP_Player.DisplayHealth` _asbp_player _output_get)
      (if (<= _output_get 0)
        (`/Game/InfiniteMatrix/Blueprints/BP_Player.DisplayRestart` _asbp_player)
        (else
          (`PrimitiveComponent.SetCollisionEnabled` OverlappedComponent "NoCollision"))))
    (:`CastFailed`
      (cast `/Game/InfiniteMatrix/Blueprints/BP_Projectile` OtherActor)
      (bind _returnvalue (`GameplayStatics.GetActorOfClass` "/Game/InfiniteMatrix/Blueprints/BP_Player.BP_Player_C"))
      (bind _output_get_2 (set `/Game/InfiniteMatrix/Blueprints/BP_Player.PlayerScore` (+ (`/Game/InfiniteMatrix/Blueprints/BP_Player.PlayerScore` _returnvalue) 1) _returnvalue))
      (`/Game/InfiniteMatrix/UI/WBP_Score.Update Score UI` (`/Game/InfiniteMatrix/Blueprints/BP_Player.ScoreWidget` _returnvalue) _output_get_2)
      (`self.K2_DestroyActor`))))

(fn `UserConstructionScript`)
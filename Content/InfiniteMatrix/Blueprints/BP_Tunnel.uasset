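; BP_Tunnel is an endless-tunnel segment with a spinning holed wall that costs the player health on contact.
; Randomize functions choose the wall's mesh and roll, and spawn an optional health pack and enemies, using square-root bounds on height for a circular cross-section.
; The trigger zone has TunnelSpawner spawn another segment, scores a point if HasClearedWall holds, then destroys this segment and its spawned actors.
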(event `self.ReceiveTick`
  (params (DeltaSeconds :type "Float (single-precision)"))
  (`SceneComponent.K2_AddLocalRotation` (`self.WallMesh`) (`KismetMathLibrary.MakeRotator` (* DeltaSeconds (`self.RotateSpeed`))) false false))

(event `self.TriggerZone.OnComponentBeginOverlap`
  (params (OverlappedComponent :type "PrimitiveComponent Object Reference") (OtherActor :type "Actor Object Reference") (OtherComp :type "PrimitiveComponent Object Reference") (OtherBodyIndex :type Integer) (bFromSweep :type Boolean) (SweepResult :type "HitResult Structure (by ref)"))
  (bind _healthpack (`self.HealthPack`))
  (bind _asbp_player (cast `/Game/InfiniteMatrix/Blueprints/BP_Player` OtherActor))
  (`/Game/InfiniteMatrix/Blueprints/BP_TunnelSpawner.SpawnTunnelAtSpawnPoint` (`self.TunnelSpawner`))
  (if (`self.HasClearedWall`)
    (bind _output_get (set `/Game/InfiniteMatrix/Blueprints/BP_Player.PlayerScore` (+ (`/Game/InfiniteMatrix/Blueprints/BP_Player.PlayerScore` _asbp_player) 1) _asbp_player))
    (`/Game/InfiniteMatrix/UI/WBP_Score.Update Score UI` (`/Game/InfiniteMatrix/Blueprints/BP_Player.ScoreWidget` _asbp_player) _output_get))
  (if (`KismetSystemLibrary.IsValid` _healthpack)
    (`self.K2_DestroyActor` _healthpack))
  (for _array_element (`self.Enemies`)
    (if (`KismetSystemLibrary.IsValid` _array_element)
      (`self.K2_DestroyActor` _array_element)))
  (`self.K2_DestroyActor`))

(event `self.WallMesh.OnComponentBeginOverlap`
  (params (OverlappedComponent :type "PrimitiveComponent Object Reference") (OtherActor :type "Actor Object Reference") (OtherComp :type "PrimitiveComponent Object Reference") (OtherBodyIndex :type Integer) (bFromSweep :type Boolean) (SweepResult :type "HitResult Structure (by ref)"))
  (bind _asbp_player (cast `/Game/InfiniteMatrix/Blueprints/BP_Player` OtherActor))
  (set `self.HasClearedWall` false)
  (bind _output_get (set `/Game/InfiniteMatrix/Blueprints/BP_Player.PlayerHealth` (- (`/Game/InfiniteMatrix/Blueprints/BP_Player.PlayerHealth` _asbp_player) 1) _asbp_player))
  (`/Game/InfiniteMatrix/Blueprints/BP_Player.DisplayHealth` _asbp_player _output_get)
  (if (<= _output_get 0)
    (`/Game/InfiniteMatrix/Blueprints/BP_Player.DisplayRestart` _asbp_player)
    (else
      (`PrimitiveComponent.SetCollisionEnabled` (`self.WallMesh`) "NoCollision"))))

(fn `RandomizeEnemy`
  (bind _returnvalue_location (`KismetMathLibrary.BreakTransform` (`self.GetTransform`)))
  (bind _returnvalue (`KismetMathLibrary.RandomFloatInRange` -400.0 400.0))
  (bind _returnvalue_2 (`KismetMathLibrary.Sqrt` (- 160000.0 (`KismetMathLibrary.MultiplyMultiply_FloatFloat` _returnvalue 2.0))))
  (for _ (range (+ (`KismetMathLibrary.RandomIntegerInRange` 0 3) 1))
    (bind _returnvalue_3 (`|SpawnActorFromClass` "/Game/InfiniteMatrix/Blueprints/BP_Enemy.BP_Enemy_C" (`KismetMathLibrary.MakeTransform` (+ (`KismetMathLibrary.MakeVector` (`KismetMathLibrary.RandomFloatInRange` 500.0 2000.0) _returnvalue (`KismetMathLibrary.RandomFloatInRange` (* _returnvalue_2 -1.0) _returnvalue_2)) _returnvalue_location)) "AdjustIfPossibleButAlwaysSpawn" "MultiplyWithRoot" null null))
    (`KismetArrayLibrary.Array_Add` (`self.Enemies`) _returnvalue_3)))

(fn `RandomizeHealthPack`
  (bind _returnvalue_location (`KismetMathLibrary.BreakTransform` (`self.GetTransform`)))
  (bind _returnvalue (`KismetMathLibrary.RandomFloatInRange` -400.0 400.0))
  (bind _returnvalue_2 (`KismetMathLibrary.Sqrt` (- 160000.0 (`KismetMathLibrary.MultiplyMultiply_FloatFloat` _returnvalue 2.0))))
  (if (`KismetMathLibrary.RandomBool`)
    (bind _returnvalue_3 (`|SpawnActorFromClass` "/Game/InfiniteMatrix/Blueprints/BP_HealthPack.BP_HealthPack_C" (`KismetMathLibrary.MakeTransform` (+ (`KismetMathLibrary.MakeVector` (`KismetMathLibrary.RandomFloatInRange` 500.0 2000.0) _returnvalue (`KismetMathLibrary.RandomFloatInRange` (* _returnvalue_2 -1.0) _returnvalue_2)) _returnvalue_location) (struct) (2.0 2.0 2.0)) "Undefined" "MultiplyWithRoot" null null))
    (set `self.HealthPack` _returnvalue_3)))

(fn `RandomizeWall`
  (`StaticMeshComponent.SetStaticMesh` (`self.WallMesh`) (select `int` (`KismetMathLibrary.RandomIntegerInRange` 0 3) :`0` "/Game/InfiniteMatrix/Meshes/SM_Hole_01.SM_Hole_01" :`1` "/Game/InfiniteMatrix/Meshes/SM_Hole_02.SM_Hole_02" :`2` "/Game/InfiniteMatrix/Meshes/SM_Hole_03.SM_Hole_03" :`3` "/Game/InfiniteMatrix/Meshes/SM_Hole_04.SM_Hole_04" :!type "StaticMesh Object Reference"))
  (`SceneComponent.K2_AddLocalRotation` (`self.WallMesh`) (`KismetMathLibrary.MakeRotator` (`KismetMathLibrary.RandomFloatInRange` 0.0 360.0)) false false))

(fn `UserConstructionScript`)